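; BP_Player is the player Blueprint that handles mouse-toggled camera look through Enhanced Input.
; BeginPlay adds the IMC_Default mapping context, and IA_Look drives controller yaw and pitch while Flag is false.
; Each look update then resets the control rotation's roll to zero, keeping pitch and yaw.
; Left mouse presses toggle Flag, switching look input on and off.
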(event Input|EnhancedActionEvents|EnhancedInputActionIA_Look
  (params (ActionValue :type Vector%202D%20Structure) (ElapsedSeconds :type Float%20%28double-precision%29) (TriggeredSeconds :type Float%20%28double-precision%29) (InputAction :type Input%20Action%20Object%20Reference :default "/Game/ThirdPerson/Input/Actions/IA_Look.IA_Look"))
  (bind (_x _y) (Math|Vector2D|BreakVector2D ActionValue))
  (bind _returnvalue (Pawn|GetControlRotation :!class /Script/Engine.Pawn))
  (bind (_roll _pitch _yaw) (Math|Rotator|BreakRotator _returnvalue))
  ;[1 1 1] コントローラーの角度を変更する
  (if (== (Variables|Default|Getflag) false)
    (Utilities|FlowControl|Sequence
      (:then_0
        (Pawn|Input|AddControllerYawInput _x)
        (Pawn|Input|AddControllerPitchInput _y))
      (:then_1
        ;[1 1 1] カメラの操作を制限する
        (Pawn|SetControlRotation (Game|GetPlayerController 0) (Math|Rotator|MakeRotator 0.0 _pitch _yaw))))))

(event EventBeginPlay
  (bind _returnvalue (Game|GetPlayerController 0))
  (bind _returnvalue_2 (PlayerController|LocalPlayerSubsystems|GetEnhancedInputLocalPlayerSubsystem _returnvalue))
  ;[1 1 1] InputをIM_Controlに設定
  (Utilities|IsValid _returnvalue_2
    (:Is%20Valid
      (Input|AddMappingContext _returnvalue_2 "/Game/ThirdPerson/Input/IMC_Default.IMC_Default" 0 "(bIgnoreAllPressedKeysUntilRelease=True,bForceImmediately=False,bNotifyUserSettings=False)"))))

(event Collision|EventActorBeginOverlap
  (params (OtherActor :type Actor%20Object%20Reference)))

(event EventTick
  (params (DeltaSeconds :type Float%20%28single-precision%29)))

(event Input|MouseEvents|LeftMouseButton
  (params (Key :type Key%20Structure :default "None"))
  (:Pressed
    (if (Variables|Default|Getflag)
      (Variables|Default|Setflag false)
      (else
        (Variables|Default|Setflag true)))))

(fn ConstructionScript)