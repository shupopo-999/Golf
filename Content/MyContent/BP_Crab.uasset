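; BP_Crab is a crab actor with a mesh component, SMCrab, that responds to vertical mouse input.
; On BeginPlay it finds BP_Player, clears its Flag and prints a debug greeting through a hardcoded true branch, leaving the mesh-visibility branch unreachable.
; The MouseY axis event sets the mesh's relative X location to the scaled axis value, replacing the position rather than accumulating it.
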(event EventBeginPlay
  (bind _returnvalue (Actor|GetActorOfClass "/Game/MyContent/BP_Player.BP_Player_C"))
  (bind _output_get (Variables|/Game/MyContent/BP_Player.BP_Player_C|Setflag _returnvalue false))
  (if true
    (Utilities|FlowControl|Sequence
      (:then_0
        (Development|PrintString "Hello")))
    (else
      (Rendering|SetVisibility (Variables|Default|GetSM_Crab) (!= _output_get false) false))))

(event Collision|EventActorBeginOverlap
  (params (OtherActor :type Actor%20Object%20Reference)))

(event EventTick
  (params (DeltaSeconds :type Float%20%28single-precision%29)))

(event Input|MouseEvents|MouseY
  (params (AxisValue :type Float%20%28single-precision%29))
  (Transformation|SetRelativeLocation (Variables|Default|GetSM_Crab) (Math|Vector|MakeVector (* AxisValue 1e+01) 0.0 0.0) false false))

(fn ConstructionScript)